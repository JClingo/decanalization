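; Harvestable resource actor that hides when overlapped, reports its homeostatic impact and harvest to BP_GameMode, and reappears on a timer started at overlap end.
; SetImpact_Event draws base impact from the game mode's random stream; toggling canalization switches between base and maximum impact.
; A dynamic material on the cylinder shows impact and decanalization as color.
; Game mode reset restores base impact, overlap count, color and visibility.
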(event `self.ReceiveBeginPlay`
  (`|ExecutionSequence`
    (:`then_0`
      (bind _asbp_game_mode (cast `/Game/Agent/BP_GameMode` (`GameplayStatics.GetGameMode`)))
      (set `self.BP Game Mode` _asbp_game_mode))
    (:`then_2`
      (bind _returnvalue (`PrimitiveComponent.CreateDynamicMaterialInstance` (`self.Cylinder`) 0 null "None"))
      (set `self.DynamicMat` _returnvalue))
    (:`then_3`
      (add `/Game/Agent/BP_GameMode.Reset` (`self.BP Game Mode`) (delegate `ResetEvent`)))
    (:`then_4`
      (add `/Game/Agent/BP_GameMode.CanalizationToggled` (`self.BP Game Mode`) (delegate `CanalizationToggled_Event`)))))

(event `ResetEvent`
  (params (ResetTransform :type Boolean))
  (`KismetSystemLibrary.K2_ClearTimer` self "Respawn")
  (set `self.HomeostaticImpact` (`self.BaseHomeostaticImpact`))
  (set `self.OverlapCount` 0)
  (`MaterialInstanceDynamic.SetVectorParameterValue` (`self.DynamicMat`) "Color" (make `LinearColor` 0.0 1.0 0.0 1.0))
  (`self.SetActorHiddenInGame` false :!label _label)
  (set `PrimitiveComponent.bGenerateOverlapEvents` true (`self.Cylinder`))
  (`self.SetActorEnableCollision` true))

(event `CanalizationToggled_Event`
  (if (`/Game/Agent/BP_GameMode.IsDecanalized` (`self.BP Game Mode`))
    (set `self.HomeostaticImpact` (`self.MaxHomeostaticImpact`))
    (else
      (set `self.HomeostaticImpact` (`self.BaseHomeostaticImpact`))))
  (`self.UpdateColor`))

(event `self.ReceiveActorBeginOverlap`
  (params (OtherActor :type "Actor Object Reference"))
  (`|ExecutionSequence`
    (:`then_0`
      (`/Engine/EditorBlueprintResources/StandardMacros.IncrementInt` (`self.OverlapCount`)))
    (:`then_1`
      (`self.SetActorHiddenInGame` true))
    (:`then_2`
      (`/Game/Agent/BP_GameMode.ImpactIncurred` (`self.BP Game Mode`) (`self.HomeostaticImpact`)))
    (:`then_3`
      (`/Game/Agent/BP_GameMode.ResourceHarvested` (`self.BP Game Mode`) self))))

(event `self.ReceiveActorEndOverlap`
  (params (OtherActor :type "Actor Object Reference"))
  (`|ExecutionSequence`
    (:`then_0`
      (`self.UpdateColor`))
    (:`then_1`
      (`KismetSystemLibrary.K2_SetTimerDelegate` (delegate `Respawn`) (`self.RespawnRate`)))))

(event `Respawn`
  (goto _label))

(event `SetImpact_Event`
  (bind _output_get (set `self.BaseHomeostaticImpact` (`KismetMathLibrary.RandomFloatInRangeFromStream` (`/Game/Agent/BP_GameMode.RandomStream` (`self.BP Game Mode`)) 5.0 (`self.MaxHomeostaticImpact`))))
  (set `self.HomeostaticImpact` _output_get)
  (`self.UpdateColor`))

(fn `UpdateColor`
  (`MaterialInstanceDynamic.SetVectorParameterValue` (`self.DynamicMat`) "Color" (make `LinearColor` 0.0 (/ (`self.HomeostaticImpact`) (`self.MaxHomeostaticImpact`)) (`KismetMathLibrary.Conv_BoolToDouble` (`/Game/Agent/BP_GameMode.IsDecanalized` (`self.BP Game Mode`))) (/ (`self.HomeostaticImpact`) (`self.BaseHomeostaticImpact`) 1.0))))

(fn `UserConstructionScript`)