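; Spline-based wall actor that sizes itself to the spawner grid defined in BP_GameMode.
; Construction script tiles WallMesh along the spline as spline mesh segments, with clamped tangents and custom collision channels.
; BeginPlay scales the actor by grid width and moves five spline points into a square from the world origin.
; It then re-stretches only the last created segment between the spline's endpoints, without rebuilding the others.
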(event `self.ReceiveBeginPlay`
  (bind _spline (`self.Spline`))
  (bind _spline_2 (`self.Spline`))
  (bind (_location _tangent) (`SplineComponent.GetLocationAndTangentAtSplinePoint` _spline_2 0 "Local"))
  (bind (_location_2 _tangent_2) (`SplineComponent.GetLocationAndTangentAtSplinePoint` _spline_2 (- (`SplineComponent.GetNumberOfSplinePoints` (`self.Spline`)) 1) "Local"))
  (bind _asbp_game_mode (cast `/Game/Agent/BP_GameMode` (`GameplayStatics.GetGameMode`)))
  (bind _spawnergridwidth (`/Game/Agent/BP_GameMode.SpawnerGridWidth` _asbp_game_mode))
  (bind _returnvalue (`KismetMathLibrary.Conv_IntToDouble` _spawnergridwidth))
  (`self.SetActorScale3D` self (`KismetMathLibrary.MakeVector` _returnvalue _returnvalue 10.0))
  (`SplineComponent.SetLocationAtSplinePoint` _spline 0 (0.0 0.0 0.0) "World" false)
  (bind _returnvalue_2 (`KismetMathLibrary.Conv_IntToDouble` (* _spawnergridwidth (`/Game/Agent/BP_GameMode.SpawnerGridSpacing` _asbp_game_mode))))
  (`SplineComponent.SetLocationAtSplinePoint` _spline 1 (`KismetMathLibrary.MakeVector` _returnvalue_2) "World" false)
  (`SplineComponent.SetLocationAtSplinePoint` _spline 2 (`KismetMathLibrary.MakeVector` _returnvalue_2 _returnvalue_2) "World" false)
  (`SplineComponent.SetLocationAtSplinePoint` _spline 3 (`KismetMathLibrary.MakeVector` 0.0 _returnvalue_2) "World" false)
  (`SplineComponent.SetLocationAtSplinePoint` _spline 4 (0.0 0.0 0.0) "World" true)
  (`SplineMeshComponent.SetStartAndEnd` (`self.SplineMesh`) _location _tangent _location_2 _tangent_2 true))

(fn `UserConstructionScript`
  (bind _xlength (`self.XLength`))
  (bind _splinemesh (`self.SplineMesh`))
  (bind _spline (`self.Spline`))
  (bind (_returnvalue_min _returnvalue_max) (break `Box` (`StaticMesh.GetBoundingBox` (`self.WallMesh`))))
  (bind _returnvalue_x (`KismetMathLibrary.BreakVector` (+ (`KismetMathLibrary.Vector_GetAbs` _returnvalue_min) (`KismetMathLibrary.Vector_GetAbs` _returnvalue_max))))
  (`PrimitiveComponent.SetCollisionObjectType` (`self.Spline`) "ECC_GameTraceChannel5")
  (bind _output_get (set `self.XLength` _returnvalue_x))
  (for _index (range (+ (`KismetMathLibrary.FTrunc` (/ (`SplineComponent.GetSplineLength` (`self.Spline`)) _output_get)) 1))
    (bind _returnvalue (`AddComponent|NODE_AddSplineMeshComponent-0` :`RelativeTransform` (`KismetMathLibrary.MakeTransform` (0.0 0.0 0.0) (struct) (1.0 1.0 0.05))))
    (`KismetArrayLibrary.Array_Add` (`self.SplineMeshes`) _returnvalue)
    (set `self.SplineMesh` _returnvalue)
    (`PrimitiveComponent.SetCollisionEnabled` (`self.SplineMesh`) "QueryAndPhysics")
    (`PrimitiveComponent.SetCollisionEnabled` _returnvalue "QueryAndPhysics")
    (`PrimitiveComponent.SetCollisionObjectType` _returnvalue "ECC_GameTraceChannel5")
    (`SplineMeshComponent.SetForwardAxis` (`self.SplineMesh`) "X" true)
    (`StaticMeshComponent.SetStaticMesh` (`self.SplineMesh`) (`self.WallMesh`))
    (`PrimitiveComponent.SetCollisionResponseToChannel` _splinemesh "ECC_GameTraceChannel4" "ECR_Ignore")
    (`PrimitiveComponent.SetCollisionResponseToChannel` _splinemesh "ECC_GameTraceChannel3" "ECR_Ignore")
    (bind _returnvalue_2 (* _index (`self.XLength`)))
    (bind _returnvalue_3 (* (+ _index 1) (`self.XLength`)))
    (`SplineMeshComponent.SetStartAndEnd` (`self.SplineMesh`) (`SplineComponent.GetLocationAtDistanceAlongSpline` _spline _returnvalue_2 "Local") (`KismetMathLibrary.ClampVectorSize` (`SplineComponent.GetTangentAtDistanceAlongSpline` _spline _returnvalue_2 "Local") 0.0 _xlength) (`SplineComponent.GetLocationAtDistanceAlongSpline` _spline _returnvalue_3 "Local") (`KismetMathLibrary.ClampVectorSize` (`SplineComponent.GetTangentAtDistanceAlongSpline` _spline _returnvalue_3 "Local") 0.0 _xlength) true)))