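; Spawner actor that scatters BP_Resource pellets over a square grid sized by the game mode.
; At BeginPlay it rolls SpawnRate per cell against the game mode's random stream to spawn the pellet pool, then positions it.
; Positioning shuffles cell indices with that stream, converts each to grid X/Y and line-traces downward to place the pellet.
; The game mode's Reset event reshuffles and repositions the existing pellets without respawning them.
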(event `self.ReceiveBeginPlay`
  (bind _gamemode (`self.GameMode`))
  (bind _spawnergridwidth (`/Game/Agent/BP_GameMode.SpawnerGridWidth` _gamemode))
  (`|ExecutionSequence`
    (:`then_0`
      (bind _asbp_game_mode (cast `/Game/Agent/BP_GameMode` (`GameplayStatics.GetGameMode`)))
      (set `self.GameMode` _asbp_game_mode))
    (:`then_1`
      (for _index (range 1 (+ (* _spawnergridwidth _spawnergridwidth) 1))
        (`KismetArrayLibrary.Array_Add` (`self.Locations`) (`KismetMathLibrary.Conv_IntToDouble` _index))))
    (:`then_2`
      (`self.SpawnResources`))
    (:`then_3`
      (add `/Game/Agent/BP_GameMode.Reset` _gamemode (delegate `Reset_Event`)))))

(event `Reset_Event`
  (params (ResetTransform :type Boolean))
  (`self.ShuffleAndPositionResources`))

(event `SpawnResources`
  (bind _spawnergridwidth (`/Game/Agent/BP_GameMode.SpawnerGridWidth` (`self.GameMode`)))
  (for _ (range 1 (+ (* _spawnergridwidth _spawnergridwidth) 1))
    ; Deprecated: Static spawn according to spawn rate
    (bind _shouldspawn (`self.ShouldSpawn` (`/Game/Agent/BP_GameMode.RandomStream` (`self.GameMode`)) (`self.SpawnRate`)))
    (if _shouldspawn
      (bind _returnvalue (`|SpawnActorFromClass` "/Game/Resource/BP_Resource.BP_Resource_C" (`KismetMathLibrary.MakeTransform` (0.0 0.0 0.0)) "AlwaysSpawn" "MultiplyWithRoot" null "" null)) ; Spawn into initial locations
      (`KismetArrayLibrary.Array_Add` (`self.Pellets`) _returnvalue)))
  (`self.ShuffleAndPositionResources`))

(event `ShuffleAndPositionResources`
  (bind (_returnvalue_x _returnvalue_y _returnvalue_z) (`KismetMathLibrary.BreakVector` (`self.K2_GetActorLocation`)))
  (bind _spawnergridspacing (`/Game/Agent/BP_GameMode.SpawnerGridSpacing` (`self.GameMode`)))
  (bind _returnvalue (/ (`KismetMathLibrary.Conv_IntToDouble` _spawnergridspacing) 2.0))
  ; Loops through alll pellets and assigns them a random, non-overlapping location (known issue: some spawning outside grid)
  (`|ExecutionSequence`
    (:`then_0`
      (`self.ShuffleLocations`))
    (:`then_1`
      (for (_array_element _array_index) (`self.Pellets`)
        (bind (_remainder _returnvalue_2) (`KismetMathLibrary.FMod` (`|GetArrayItem` (`self.Locations`) _array_index) (`KismetMathLibrary.Conv_IntToDouble` (`/Game/Agent/BP_GameMode.SpawnerGridWidth` (`self.GameMode`)))))
        (bind _returnvalue_3 (`KismetMathLibrary.MakeVector` (+ _returnvalue (`KismetMathLibrary.Conv_IntToDouble` (* _returnvalue_2 _spawnergridspacing))) (+ (* _spawnergridspacing _remainder) _returnvalue) _returnvalue_z))
        (bind _outhit (`KismetSystemLibrary.LineTraceSingle` _returnvalue_3 (+ _returnvalue_3 (* (`KismetMathLibrary.GetUpVector` (`self.K2_GetActorRotation`)) -5000.0)) "TraceTypeQuery3"))
        (bind (_bblockinghit _binitialoverlap _time _distance _location) (`GameplayStatics.BreakHitResult` _outhit))
        (if _bblockinghit
          (`self.K2_SetActorLocation` _array_element _location false true)
          (`/Game/Resource/BP_Resource.SetImpact_Event` _array_element))))))

(fn `ShouldSpawn`
  (params (RandomStream :type "RandomStream Structure (by ref)") (SpawnRate :type "Float (double-precision)"))
  (returns (ShouldSpawn :type Boolean))
  (return (`KismetMathLibrary.RandomBoolWithWeightFromStream` RandomStream SpawnRate)))

(fn `ShuffleLocations`
  (`KismetArrayLibrary.Array_ShuffleFromStream` (`self.Locations`) (`/Game/Agent/BP_GameMode.RandomStream` (`self.GameMode`))))

(fn `UserConstructionScript`)