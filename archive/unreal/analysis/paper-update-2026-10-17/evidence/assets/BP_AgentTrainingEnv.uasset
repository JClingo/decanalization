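; Learning Agents training environment that scores BP_Agent on keeping a homeostatic setpoint value near zero.
; GatherAgentReward reads GameMode history, using either homeostatic or older delta/exponential formulas, each split into HRL and LM (deficit-focused) variants; many unwired experiments remain.
; Straying beyond MaxSetpointDistance flags termination, while exceeding MaxTime truncates.
; Episode reset reports total reward and setpoint standard deviation to GameMode, then resets state and agent.
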(fn `GatherAgentCompletion`
  (params (AgentId :type Integer))
  (returns (OutCompletion :type "ELearningAgentsCompletion Enum"))
  (if (`self.ShouldTerminate`)
    (`KismetSystemLibrary.PrintString` null "Termination")
    (return (`LearningAgentsCompletions.MakeCompletion` "Termination" "Completion" false null))
    (elif (> (`self.GetEpisodeTime` AgentId) (`self.Max Time`))
      (`KismetSystemLibrary.PrintString` null "Truncation")
      (return (`LearningAgentsCompletions.MakeCompletion` "Truncation" "Completion" false null))
      (else
        (return "Running")))))

(fn `GatherAgentReward`
  (params (AgentId :type Integer))
  (returns (OutReward :type "Float (single-precision)"))
  (locals (Agent :type "/Game/Agent/BP_Agent Object Reference") (CurrentReward :type "Float (double-precision)") (StdDev :type "Float (double-precision)") (EpisodeNet :type "Float (double-precision)") (EpisodeSetpoint :type "Float (double-precision)"))
  (bind _value (`self.GetPreviousSetpoint`))
  (bind _setpoint (`self.GetCurrentSetpoint`))
  (bind _setpoint_2 (`self.GetCurrentSetpoint`))
  (bind _totalreward (`self.TotalReward`))
  (bind _gamemode (`self.GameMode`))
  (bind _currentreward (`local.CurrentReward`))
  (bind _shouldterminate (`self.ShouldTerminate`))
  (bind _episode_steps (`self.Episode Steps`))
  (bind _returnvalue (`KismetMathLibrary.Abs` (`self.GetPreviousSetpoint`)))
  (bind _returnvalue_2 (`KismetMathLibrary.Abs` (`self.GetCurrentSetpoint`)))
  (bind _returnvalue_3 (`KismetMathLibrary.Abs` _setpoint_2))
  (bind _returnvalue_4 (`KismetMathLibrary.Abs` (`self.GetCurrentSetpoint`)))
  (bind _returnvalue_5 (`KismetMathLibrary.FMax` (`self.HomeostaticRewardRate`)))
  (bind _returnvalue_6 (`KismetMathLibrary.FMax` (`self.RewardDistanceScale`) 0.001))
  (bind _ishrl (`/Game/Agent/BP_GameMode.IsHRL` (`self.GameMode`)))
  (bind _returnvalue_7 (/ _returnvalue_4 _returnvalue_6))
  (bind _returnvalue_8 (- _returnvalue _returnvalue_2))
  (bind _returnvalue_9 (> _returnvalue_4 (`self.Max Setpoint Distance`)))
  ; Calculate Rewards
  (if (`self.UseHomeostaticReward`)
    (if _shouldterminate
      (return 0.0) ; Post-end episode (this doesn't immediately pick up completions)
      (else
        (if _returnvalue_9
          (set `self.ShouldTerminate` true)
          (if _ishrl
            (set `local.CurrentReward` (`KismetMathLibrary.FMin` (`self.HomeostaticFailureReward`)))
            (else
              (set `local.CurrentReward` 0.0 :!label _label)))
          (elif _ishrl
            (set `local.CurrentReward` (* (/ _returnvalue_5 (+ 1.0 (* _returnvalue_7 _returnvalue_7))) (`GameplayStatics.GetWorldDeltaSeconds` _gamemode)))
            (elif (< _setpoint 0.0)
              (set `local.CurrentReward` (* (/ (`KismetMathLibrary.FMax` (- (`KismetMathLibrary.Abs` (`KismetMathLibrary.SelectFloat` (`self.PreviousRewardState`) _value (`self.HasPreviousRewardState`))) (`KismetMathLibrary.Abs` _setpoint))) _returnvalue_6) _returnvalue_5))
              (else
                (goto _label)))))
        ; HRL-Collision Reward
        (set `self.TotalReward` (+ _totalreward _currentreward))
        (set `self.PreviousRewardState` _setpoint)
        (set `self.HasPreviousRewardState` true)
        (set `self.Episode Steps` (+ _episode_steps 1))
        (return _currentreward)))
    (elif (not _shouldterminate)
      ; Common initialization
      (if _returnvalue_9
        (set `self.ShouldTerminate` true)
        (return 0.0) ; Prematurely hit setpoint limit!
        (else
          (set `local.Agent` (`self.GetAgent` AgentId "/Game/Agent/BP_Agent.BP_Agent_C"))
          (`/Engine/EditorBlueprintResources/StandardMacros.IncrementInt` _episode_steps
            (:`  `
              (`|ExecutionSequence`
                (:`then_0`
                  ;;[0 0.06125 0.0137] For setpoints and anticipated net, need to be sure there's a difference between this and the past measurement (otherwise we just ignore it)
                  (if (or (== (`self.GetPreviousSetpoint`) (`self.GetCurrentSetpoint`)) (== (`self.GetCurrentNet`) (`self.GetPreviousNet`)))
                    (return 0.0)))
                (:`then_1`
                  (if (`/Game/Agent/BP_GameMode.IsHRL` (`self.GameMode`))
                    ;; HRL - Simple Pre vs post - did we get closer or farther between timesteps?
                    (if (> (- (`KismetMathLibrary.Abs` (`self.GetPreviousSetpoint`)) (`KismetMathLibrary.Abs` _setpoint_2)) 0.0)
                      (set `local.CurrentReward` (+ (`LearningAgentsRewards.MakeReward` (`KismetMathLibrary.MultiplyMultiply_FloatFloat` 2.718282 (* 0.005 _returnvalue_3 -1.0)) 1.0 "Reward" true null) (`local.CurrentReward`)))
                      (else
                        (set `local.CurrentReward` (+ (`LearningAgentsRewards.MakeReward` (- 1.0 (`KismetMathLibrary.MultiplyMultiply_FloatFloat` 2.718282 (* 0.0001 _returnvalue_3))) 1.0 "Reward" true null) (`local.CurrentReward`)))))
                    (else
                      ;; LM-Just based on previous vs current
                      (if (and (>= (`self.GetPreviousSetpoint`) 0.0) (>= (`self.GetCurrentSetpoint`) 0.0))
                        _
                        (elif (and (>= (`self.GetPreviousSetpoint`) 0.0) (< (`self.GetCurrentSetpoint`) 0.0))
                          (set `local.CurrentReward` (+ (`LearningAgentsRewards.MakeReward` _setpoint 1.0 "Reward" true null) (`local.CurrentReward`)))
                          (elif (and (< _value 0.0) (>= (`self.GetCurrentSetpoint`) 0.0))
                            (set `local.CurrentReward` (+ (`LearningAgentsRewards.MakeReward` (`KismetMathLibrary.Abs` (`self.GetPreviousSetpoint`)) (`/Game/Agent/BP_GameMode.AlphaNF` _gamemode) "Reward" true null) (`local.CurrentReward`)))
                            (elif (> _returnvalue_2 _returnvalue)
                              (set `local.CurrentReward` (+ (`LearningAgentsRewards.MakeReward` _returnvalue_8 1.0 "Reward" true null) (`local.CurrentReward`)))
                              (else
                                (set `local.CurrentReward` (+ (`LearningAgentsRewards.MakeReward` _returnvalue_8 (`/Game/Agent/BP_GameMode.AlphaNF` (`self.GameMode`)) "Reward" true null) (`local.CurrentReward`)))))))))))
                (:`then_3`
                  (bind _output_get (set `self.TotalReward` (+ (`local.CurrentReward`) _totalreward)))
                  (return (`local.CurrentReward`))))))))
      (else
        (return 0.0) ; Post-end episode (this doesn't immediately pick up completions)
      ))))

(fn `GetCurrentNet`
  (returns (Net :type "Float (double-precision)"))
  (bind _anticipatednets (`/Game/Agent/BP_GameMode.AnticipatedNets` (`self.GameMode`)))
  (return (`|GetArrayItem` _anticipatednets (`KismetArrayLibrary.Array_LastIndex` _anticipatednets))))

(fn `GetCurrentSetpoint`
  (returns (setpoint :type "Float (double-precision)"))
  (bind _setpoints (`/Game/Agent/BP_GameMode.Setpoints` (`self.GameMode`)))
  (return (`|GetArrayItem` _setpoints (`KismetArrayLibrary.Array_LastIndex` _setpoints))))

(fn `GetPreviousNet`
  (returns (Net :type "Float (double-precision)"))
  (bind _anticipatednets (`/Game/Agent/BP_GameMode.AnticipatedNets` (`self.GameMode`)))
  (if (> (`KismetArrayLibrary.Array_Length` _anticipatednets) 1)
    (return (`|GetArrayItem` _anticipatednets (- (`KismetArrayLibrary.Array_LastIndex` _anticipatednets) 1)))
    (else
      (return 0.0))))

(fn `GetPreviousSetpoint`
  (returns (Value :type "Float (double-precision)"))
  (bind _setpoints (`/Game/Agent/BP_GameMode.Setpoints` (`self.GameMode`)))
  (return (`|GetArrayItem` _setpoints (`KismetMathLibrary.Max` (- (`KismetArrayLibrary.Array_LastIndex` _setpoints) 1)))))

(fn `GetStandardDeviation`
  (params (Values :type "Array of Float (double-precision)"))
  (returns (StdDev :type "Float (double-precision)"))
  (locals (Total :type "Float (double-precision)") (Mean :type "Float (double-precision)") (Variance :type "Float (double-precision)"))
  (if (== (`KismetArrayLibrary.Array_Length` Values) 0)
    (return 0.0)
    (else
      (for _array_element Values
        (set `local.Total` (+ _array_element (`local.Total`))))
      (set `local.Mean` (/ (`local.Total`) (`KismetMathLibrary.Conv_IntToDouble` (`KismetArrayLibrary.Array_Length` Values))))
      (for _array_element_2 Values
        (set `local.Variance` (+ (`local.Variance`) (`KismetMathLibrary.MultiplyMultiply_FloatFloat` (- _array_element_2 (`local.Mean`)) 2.0))))
      (return (`KismetMathLibrary.Sqrt` (`local.Variance`))))))

(fn `Initialize`
  (params (`Game Mode` :type "/Game/Agent/BP_GameMode Object Reference"))
  (set `self.Episode Steps` 0)
  (set `self.TotalReward` 0.0)
  (set `self.ShouldTerminate` false)
  (set `self.LastCollidingResource` null)
  (set `self.HasPreviousRewardState` false)
  (set `self.PreviousRewardState` 0.0)
  (return))

(fn `ResetAgentEpisode`
  (params (AgentId :type Integer))
  (if (> (`self.Episode Steps`) 1)
    (`/Game/Agent/BP_GameMode.LearningEpisodeCompleted` (`self.GameMode`) (`self.TotalReward`) (`self.GetStandardDeviation` (`/Game/Agent/BP_GameMode.Setpoints` (`self.GameMode`)))))
  (`self.Initialize` (`self.GameMode`))
  (`/Game/Agent/BP_Agent.Reset` (`self.GetAgent` AgentId "/Game/Agent/BP_Agent.BP_Agent_C")))