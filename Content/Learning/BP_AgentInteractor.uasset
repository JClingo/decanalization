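; Learning Agents interactor for BP_Agent that defines what the agent observes and how it acts in a homeostatic drive-reduction task.
; Observations combine a forward fan of drive-reduction ray traces, the game mode's latest setpoint, a resource-collision flag and anticipated resource gain and loss.
; The only action is a "Look" float applied as controller yaw input.
; Drive-increase tile rays and drive totals remain in the graph but never run.
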(fn `GatherAgentObservation`
  (params (InObservationObject :type "LearningAgentsObservationObject Object Reference") (AgentId :type Integer))
  (returns (OutObservationObjectElement :type "LearningAgentsObservationObjectElement Structure"))
  (locals (ObsActor :type "/Game/Agent/BP_Agent Object Reference") (AgId :type Integer :default 0) (DriveReductionRayObs :type "Array of LearningAgentsObservationObjectElement Structure") (DriveIncreaseRayObs :type "Array of LearningAgentsObservationObjectElement Structure") (DriveReductionTotal :type "Float (double-precision)") (DriveIncreaseTotal :type "Float (double-precision)") (DistanceSample :type "Float (double-precision)"))
  (bind _obsactor (`local.ObsActor`))
  (bind _returnvalue (`Actor.K2_GetActorLocation` (`local.ObsActor`)))
  (bind _setpoints (`/Game/Agent/BP_GameMode.Setpoints` (`/Game/Agent/BP_Agent.BP Game Mode` (`local.ObsActor`))))
  (set `local.AgId` AgentId)
  (set `local.ObsActor` (`self.GetAgent` AgentId "/Game/Agent/BP_Agent.BP_Agent_C"))
  (`|ExecutionSequence`
    (:`then_0`
      (`|ExecutionSequence`
        (:`then_1`
          ; Populate Resource Object Observations
          (`KismetArrayLibrary.Array_Clear` (`local.DriveReductionRayObs`))
          (for _index (range 7)
            (`KismetArrayLibrary.Array_Add` (`local.DriveReductionRayObs`) (`LearningAgentsObservations.MakeProportionAlongRayObservation` (`local.InObservationObject`) (0.0 0.0 0.0) (`KismetMathLibrary.RotateAngleAxis` (* (`KismetMathLibrary.GetForwardVector` (`KismetMathLibrary.MakeRotator` 0.0 0.0 (.yaw (`Actor.K2_GetActorRotation` (`local.ObsActor`))))) (`/Game/Agent/BP_Agent.HorizonLength` (`local.ObsActor`))) (`|GetArrayItem` (`|MakeArray` -45.0 -22.5 -11.7 0.0 11.7 22.5 45.0) _index) (`KismetMathLibrary.Vector_Up`)) (`KismetMathLibrary.MakeTransform` _returnvalue) "ECC_GameTraceChannel3" "ProportionAlongRayObservation" true null (`local.AgId`) _returnvalue))))))
    (:`then_3`
      (return (`LearningAgentsObservations.MakeStructObservation` (`local.InObservationObject`) (`|MakeMap` "DriveReductionRays" (`LearningAgentsObservations.MakeStaticArrayObservation` (`local.InObservationObject`) (`local.DriveReductionRayObs`)) "SetpointDistance" (`LearningAgentsObservations.MakeFloatObservation` (`local.InObservationObject`) (`KismetArrayLibrary.Array_Get` _setpoints (`KismetArrayLibrary.Array_LastIndex` _setpoints)) "FloatObservation" false null) "DriveReductionCollision" (`LearningAgentsObservations.MakeBoolObservation` (`local.InObservationObject`) (`KismetSystemLibrary.IsValid` (`/Game/Agent/BP_Agent.CollidingResource` (`local.ObsActor`))) "BoolObservation" false null) "Perception" (`LearningAgentsObservations.MakeStructObservation` (`local.InObservationObject`) (`|MakeMap` "PerceivedLoss" (`LearningAgentsObservations.MakeFloatObservation` (`local.InObservationObject`) (`/Game/Agent/BP_Agent.AnticipatedResourceLoss` _obsactor) "FloatObservation" false null) "PerceivedGain" (`LearningAgentsObservations.MakeFloatObservation` (`local.InObservationObject`) (`/Game/Agent/BP_Agent.AnticipatedResourceGain` _obsactor) "FloatObservation" false null) :!type "Name")) :!type "Name"))))))

(fn `PerformAgentAction`
  (params (InActionObject :type "LearningAgentsActionObject Object Reference") (InActionObjectElement :type "LearningAgentsActionObjectElement Structure (by ref)") (AgentId :type Integer))
  (locals (`Action Actor` :type "/Game/Agent/BP_Agent Object Reference"))
  (set `local.Action Actor` (`self.GetAgent` AgentId "/Game/Agent/BP_Agent.BP_Agent_C"))
  (bind _outelements (`LearningAgentsActions.GetStructAction` (`local.InActionObject`) (`local.InActionObjectElement`)))
  (`|ExecutionSequence`
    (:`then_0`
      (bind _outvalue (`LearningAgentsActions.GetFloatAction` (`local.InActionObject`) (`BlueprintMapLibrary.Map_Find` _outelements "Look") "Look" true null))
      (`Pawn.AddControllerYawInput` (`local.Action Actor`) _outvalue))
    (:`then_1`
      (return))))

(fn `SpecifyAgentAction`
  (params (InActionSchema :type "LearningAgentsActionSchema Object Reference"))
  (returns (OutActionSchemaElement :type "LearningAgentsActionSchemaElement Structure"))
  (return (`LearningAgentsActions.SpecifyStructAction` (`local.InActionSchema`) (`|MakeMap` "Look" (`LearningAgentsActions.SpecifyFloatAction` (`local.InActionSchema`) 1.0 "Look") :!type "Name"))))

(fn `SpecifyAgentObservation`
  (params (InObservationSchema :type "LearningAgentsObservationSchema Object Reference"))
  (returns (OutObservationSchemaElement :type "LearningAgentsObservationSchemaElement Structure"))
  (bind _inobservationschema (`local.InObservationSchema`))
  (bind _inobservationschema_2 (`local.InObservationSchema`))
  (bind _inobservationschema_3 (`local.InObservationSchema`))
  (return (`LearningAgentsObservations.SpecifyStructObservation` (`local.InObservationSchema`) (`|MakeMap` "DriveReductionRays" (`LearningAgentsObservations.SpecifyStaticArrayObservation` _inobservationschema_3 (`LearningAgentsObservations.SpecifyProportionAlongRayObservation` _inobservationschema_3) 7) "SetpointDistance" (`LearningAgentsObservations.SpecifyFloatObservation` _inobservationschema_2 100.0) "DriveReductionCollision" (`LearningAgentsObservations.SpecifyBoolObservation` _inobservationschema_2) "Perception" (`LearningAgentsObservations.SpecifyStructObservation` (`local.InObservationSchema`) (`|MakeMap` "PerceivedLoss" (`LearningAgentsObservations.SpecifyFloatObservation` _inobservationschema 100.0) "PerceivedGain" (`LearningAgentsObservations.SpecifyFloatObservation` _inobservationschema 100.0) :!type "Name")) :!type "Name"))))