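; Learning Agents training environment for BP_Agent that scores, ends and resets reinforcement learning episodes.
; Reward combines reward-object collision with weighted proximity to three horizon raycast hits; exceeding the setpoint limit returns a large penalty and flags termination, while timeout truncates.
; Setpoint distances and their standard deviation are tracked, and reset reports total reward and deviation to the GameMode.
; Older setpoint-delta and survival reward logic remains disconnected, and batch overrides are empty.
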(fn `GatherAgentCompletion`
  (params (AgentId :type Integer))
  (returns (OutCompletion :type "ELearningAgentsCompletion Enum"))
  (return (`LearningAgentsCompletions.CompletionOr` (`LearningAgentsCompletions.MakeCompletionOnCondition` (`self.ShouldTerminate`) "Termination" "ConditionCompletion" false null) (`LearningAgentsCompletions.MakeCompletionOnTimeElapsed` (`self.GetEpisodeTime` AgentId) (`self.Max Time`) "Truncation" "TimeElapsedCompletion" false null))))

(fn `GatherAgentCompletions`
  (params (AgentIds :type "Array of Integer (by ref)"))
  (returns (OutCompletions :type "Array of ELearningAgentsCompletion Enum"))
  (return))

(fn `GatherAgentReward`
  (params (AgentId :type Integer))
  (returns (OutReward :type "Float (single-precision)"))
  (locals (RewardActor :type "/Game/Agent/BP_Agent Object Reference") (CurrentReward :type "Float (double-precision)") (AgId :type Integer :default 0) (StdDev :type "Float (double-precision)"))
  (bind _episode_steps (`self.Episode Steps`))
  (bind _episodesetpoints (`self.EpisodeSetpoints`))
  (bind _rewardactor (`local.RewardActor`))
  (bind _episodestddevs (`self.EpisodeStdDevs`))
  (bind _returnvalue (`Actor.K2_GetActorLocation` (`local.RewardActor`)))
  (bind _setpointdistance (`/Game/Agent/BP_Agent.SetpointDistance` (`local.RewardActor`)))
  (bind _returnhitpositions (`/Game/Agent/BP_Agent.FindHitLocation` _rewardactor (`/Game/Agent/BP_Agent.HorizonLength` _rewardactor) (`|MakeArray` 0.0 11.7 -11.7)))
  (bind _returnvalue_2 (+ (`LearningAgentsRewards.MakeRewardOnCondition` (`/Game/Agent/BP_Agent.IsCollidingWithReward` (`local.RewardActor`)) 10.0 "ConditionReward" false null) (`LearningAgentsRewards.MakeRewardOnLocationDifferenceBelowThreshold` _returnvalue (`|GetArrayItem` _returnhitpositions) 5000.0 0.1 "GettingCloseToReducerReward" false null) (`LearningAgentsRewards.MakeRewardOnLocationDifferenceBelowThreshold` _returnvalue (`|GetArrayItem` _returnhitpositions 1) 5000.0 0.5 "GettingCloseToReducerReward" false null) (`LearningAgentsRewards.MakeRewardOnLocationDifferenceBelowThreshold` _returnvalue (`|GetArrayItem` _returnhitpositions 2) 5000.0 0.1 "GettingCloseToReducerReward" false null)))
  (if (== _episode_steps 0)
    (`/Engine/EditorBlueprintResources/StandardMacros.IncrementInt` _episode_steps
      (:`  `
        (return 0.0)))
    (else
      (set `local.AgId` 0)
      (set `local.RewardActor` (`self.GetAgent` AgentId "/Game/Agent/BP_Agent.BP_Agent_C"))
      (`/Engine/EditorBlueprintResources/StandardMacros.IncrementInt` (`self.Episode Steps`)
        (:`  `
          (if (> (`KismetMathLibrary.Abs` _setpointdistance) (`self.Max Setpoint Distance`))
            (if (`self.ShouldTerminate`)
              (return 0.0) ; Post-end episode
              (else
                (set `self.ShouldTerminate` true)
                (return -50.0) ; Prematurely hit setpoint limit!
              ))
            (else
              (if (not (== _setpointdistance (`|GetArrayItem` _episodesetpoints (`KismetArrayLibrary.Array_LastIndex` _episodesetpoints))))
                (`KismetArrayLibrary.Array_Add` (`self.EpisodeSetpoints`) _setpointdistance)
                (bind _stddev (`self.GetStandardDeviation` (`self.EpisodeSetpoints`))))
              (if (not (== _stddev (`|GetArrayItem` _episodestddevs (`KismetArrayLibrary.Array_LastIndex` _episodestddevs))))
                (`KismetArrayLibrary.Array_Add` (`self.EpisodeStdDevs`) _stddev)
                (set `local.StdDev` _stddev))
              (`KismetSystemLibrary.PrintString` null (`KismetStringLibrary.Conv_DoubleToString` _returnvalue_2))
              (set `self.TotalReward` (+ _returnvalue_2 (`self.TotalReward`)))
              (return _returnvalue_2))))))))

(fn `GatherAgentRewards`
  (params (AgentIds :type "Array of Integer (by ref)"))
  (returns (OutRewards :type "Array of Float (single-precision)"))
  (return))

(fn `GetStandardDeviation`
  (params (Values :type "Array of Float (double-precision)"))
  (returns (StdDev :type "Float (double-precision)"))
  (locals (Total :type "Float (double-precision)") (Mean :type "Float (double-precision)") (Variance :type "Float (double-precision)"))
  (if (== (`KismetArrayLibrary.Array_Length` Values) 0)
    (return 0.0)
    (else
      (for _array_element Values
        (set `local.Total` (+ _array_element (`local.Total`))))
      (set `local.Mean` (/ (`local.Total`) (`KismetMathLibrary.Conv_IntToDouble` (`KismetArrayLibrary.Array_Length` Values))))
      (for _array_element_2 Values
        (set `local.Variance` (+ (`local.Variance`) (`KismetMathLibrary.MultiplyMultiply_FloatFloat` (- _array_element_2 (`local.Mean`)) 2.0))))
      (return (`KismetMathLibrary.Sqrt` (`local.Variance`))))))

(fn `ResetAgentEpisode`
  (params (AgentId :type Integer))
  (bind _episodestddevs (`self.EpisodeStdDevs`))
  (if (not (== (`self.Episode Steps`) 0))
    (`/Game/Agent/BP_GameMode.LearningEpisodeCompleted` (`self.GameMode`) (`self.TotalReward`) (`|GetArrayItem` _episodestddevs (`KismetArrayLibrary.Array_LastIndex` _episodestddevs)))
    (set `self.Episode Steps` 0)
    (set `self.TotalReward` 0.0)
    (`KismetArrayLibrary.Array_Clear` (`self.EpisodeSetpoints`))
    (`KismetArrayLibrary.Array_Clear` (`self.EpisodeStdDevs`))
    (set `self.ShouldTerminate` false))
  (`/Game/Agent/BP_Agent.Reset` (`self.GetAgent` AgentId "/Game/Agent/BP_Agent.BP_Agent_C")))

(fn `ResetAgentEpisodes`
  (params (AgentIds :type "Array of Integer (by ref)"))
  (return))