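; BP_ResourceManager scatters BP_Resource actors over a square grid at BeginPlay.
; It takes grid width, spacing and random stream from BP_GameMode, then rolls each cell against SpawnRate using that stream.
; Successful cells trace from their center, offset from the manager's location, 5000 units along its negative up vector on a specific trace channel.
; A resource spawns at each blocking hit.
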(event `self.ReceiveBeginPlay`
  (`|ExecutionSequence`
    (:`then_0`
      (bind _asbp_game_mode (cast `/Game/Agent/BP_GameMode` (`GameplayStatics.GetGameMode`)))
      (set `self.GameMode` _asbp_game_mode))
    (:`then_1`
      (`self.SpawnTiles`))))

(event `SpawnTiles`
  (bind (_returnvalue_x _returnvalue_y _returnvalue_z) (`KismetMathLibrary.BreakVector` (`self.K2_GetActorLocation`)))
  (bind _returnvalue_x_2 (`KismetMathLibrary.BreakVector` (`self.K2_GetActorLocation`)))
  (bind _gamemode (`self.GameMode`))
  (bind _spawnergridspacing (`/Game/Agent/BP_GameMode.SpawnerGridSpacing` _gamemode))
  (bind _spawnergridspacing_2 (`/Game/Agent/BP_GameMode.SpawnerGridSpacing` _gamemode))
  (for _index (range (`/Game/Agent/BP_GameMode.SpawnerGridWidth` _gamemode))
    (for _index_2 (range (`/Game/Agent/BP_GameMode.SpawnerGridWidth` _gamemode))
      (bind _shouldspawn (`self.ShouldSpawn` (`/Game/Agent/BP_GameMode.RandomStream` _gamemode) (`self.SpawnRate`)))
      (if _shouldspawn
        (bind _returnvalue (`KismetMathLibrary.MakeVector` (+ (* _index _spawnergridspacing) (+ _returnvalue_x_2 (* (`KismetMathLibrary.Conv_IntToDouble` _spawnergridspacing) 0.5))) (+ (* _index_2 _spawnergridspacing_2) (+ _returnvalue_y (* (`KismetMathLibrary.Conv_IntToDouble` _spawnergridspacing_2) 0.5))) _returnvalue_z))
        (bind _outhit (`KismetSystemLibrary.LineTraceSingle` _returnvalue (+ _returnvalue (* (`KismetMathLibrary.GetUpVector` (`self.K2_GetActorRotation`)) -5000.0)) "TraceTypeQuery3"))
        (bind (_bblockinghit _binitialoverlap _time _distance _location) (`GameplayStatics.BreakHitResult` _outhit))
        (if _bblockinghit
          (`|SpawnActorFromClass` "/Game/Resource/BP_Resource.BP_Resource_C" (`KismetMathLibrary.MakeTransform` _location) "AlwaysSpawn" "MultiplyWithRoot" null "" null))))))

(fn `ShouldSpawn`
  (params (RandomStream :type "RandomStream Structure (by ref)") (SpawnRate :type "Float (double-precision)"))
  (returns (ShouldSpawn :type Boolean))
  (return (`KismetMathLibrary.RandomBoolWithWeightFromStream` RandomStream SpawnRate)))

(fn `UserConstructionScript`)