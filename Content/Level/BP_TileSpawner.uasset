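; Level actor that fills a square grid with BP_Tile actors on BeginPlay, using grid width and spacing from BP_GameMode.
; Each cell center, offset from the spawner's location, gets a short downward line trace, and a tile spawns only at a blocking hit.
; After each row it measures one tile's scaled XY bounds and writes the diagonal to the game mode's TileHypotenuseLength.
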(event `self.ReceiveBeginPlay`
  (`|ExecutionSequence`
    (:`then_0`
      (bind _asbp_game_mode (cast `/Game/Agent/BP_GameMode` (`GameplayStatics.GetGameMode`)))
      (set `self.BP Game Mode` _asbp_game_mode))
    (:`then_1`
      (`self.SpawnTiles`))))

(event `SpawnTiles`
  (bind (_returnvalue_x _returnvalue_y _returnvalue_z) (`KismetMathLibrary.BreakVector` (`self.K2_GetActorLocation`)))
  (bind _returnvalue_x_2 (`KismetMathLibrary.BreakVector` (`self.K2_GetActorLocation`)))
  (bind _bp_game_mode (`self.BP Game Mode`))
  (bind _spawnergridspacing (`/Game/Agent/BP_GameMode.SpawnerGridSpacing` _bp_game_mode))
  (for _index (range (`/Game/Agent/BP_GameMode.SpawnerGridWidth` _bp_game_mode))
    (for _index_2 (range (`/Game/Agent/BP_GameMode.SpawnerGridWidth` _bp_game_mode))
      (bind _returnvalue (`KismetMathLibrary.MakeVector` (+ (* _index _spawnergridspacing) (+ _returnvalue_x_2 (* (`KismetMathLibrary.Conv_IntToDouble` _spawnergridspacing) 0.5))) (+ (* _index_2 _spawnergridspacing) (+ _returnvalue_y (* (`KismetMathLibrary.Conv_IntToDouble` _spawnergridspacing) 0.5))) _returnvalue_z))
      (bind _outhit (`KismetSystemLibrary.LineTraceSingle` _returnvalue (+ _returnvalue (* (`KismetMathLibrary.GetUpVector` (`self.K2_GetActorRotation`)) -500.0)) "TraceTypeQuery3"))
      (bind (_bblockinghit _binitialoverlap _time _distance _location) (`GameplayStatics.BreakHitResult` _outhit))
      (if _bblockinghit
        (`|SpawnActorFromClass` "/Game/Level/BP_Tile.BP_Tile_C" (`KismetMathLibrary.MakeTransform` _location) "Undefined" "MultiplyWithRoot" null null)))
    (bind _returnvalue_2 (`GameplayStatics.GetActorOfClass` "/Game/Level/BP_Tile.BP_Tile_C"))
    (bind _cube (`/Game/Level/BP_Tile.Cube` _returnvalue_2))
    (bind (_relativescale3d_x _relativescale3d_y) (`KismetMathLibrary.BreakVector` (`SceneComponent.RelativeScale3D` _cube)))
    (bind (_min _max) (`StaticMeshComponent.GetLocalBounds` _cube))
    (bind (_returnvalue_x_3 _returnvalue_y_2) (`KismetMathLibrary.BreakVector` (- _max _min)))
    (set `/Game/Agent/BP_GameMode.TileHypotenuseLength` (`KismetMathLibrary.Sqrt` (+ (`KismetMathLibrary.Square` (* _relativescale3d_x _returnvalue_x_3)) (`KismetMathLibrary.Square` (* _returnvalue_y_2 _relativescale3d_y)))) (`self.BP Game Mode`))))

(fn `UserConstructionScript`)