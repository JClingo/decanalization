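; Level actor that builds a tall wall along an editable spline in its construction script.
; It measures the wall mesh's X length from its bounding box and chains spline mesh segments at that interval, stretched tenfold in Z.
; Tangents are clamped to segment length, and each segment gets collision that blocks one custom trace channel and ignores another.
; The event graph is empty, and a second segment setup is left unconnected.
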(event `self.ReceiveActorBeginOverlap`
  (params (OtherActor :type "Actor Object Reference")))

(fn `UserConstructionScript`
  (bind _spline (`self.Spline`))
  (bind _spline_2 (`self.Spline`))
  (bind _xlength (`self.XLength`))
  (bind (_returnvalue_min _returnvalue_max) (break `Box` (`StaticMesh.GetBoundingBox` (`self.WallMesh`))))
  (bind _returnvalue_x (`KismetMathLibrary.BreakVector` (+ (`KismetMathLibrary.Vector_GetAbs` _returnvalue_min) (`KismetMathLibrary.Vector_GetAbs` _returnvalue_max))))
  (`PrimitiveComponent.SetCollisionObjectType` (`self.Spline`) "ECC_GameTraceChannel5")
  (bind _output_get (set `self.XLength` _returnvalue_x))
  (for _index (range (+ (`KismetMathLibrary.FTrunc` (/ (`SplineComponent.GetSplineLength` (`self.Spline`)) _output_get)) 1))
    (bind _returnvalue (`AddComponent|NODE_AddSplineMeshComponent-0` :`RelativeTransform` (`KismetMathLibrary.MakeTransform` (0.0 0.0 0.0) (struct) (1.0 1.0 10.0))))
    (set `self.SplineMesh` _returnvalue)
    (`PrimitiveComponent.SetCollisionEnabled` _returnvalue "QueryAndPhysics")
    (`PrimitiveComponent.SetCollisionEnabled` (`self.SplineMesh`) "QueryAndPhysics")
    (`SplineMeshComponent.SetForwardAxis` (`self.SplineMesh`) "X" true)
    (`StaticMeshComponent.SetStaticMesh` (`self.SplineMesh`) (`self.WallMesh`))
    (`PrimitiveComponent.SetCollisionResponseToChannel` (`self.SplineMesh`) "ECC_GameTraceChannel5" "ECR_Block")
    (`PrimitiveComponent.SetCollisionResponseToChannel` (`self.SplineMesh`) "ECC_GameTraceChannel4" "ECR_Ignore")
    (bind _returnvalue_2 (* _index (`self.XLength`)))
    (bind _returnvalue_3 (* (+ _index 1) (`self.XLength`)))
    (`SplineMeshComponent.SetStartAndEnd` (`self.SplineMesh`) (`SplineComponent.GetLocationAtDistanceAlongSpline` _spline_2 _returnvalue_2 "Local") (`KismetMathLibrary.ClampVectorSize` (`SplineComponent.GetTangentAtDistanceAlongSpline` _spline_2 _returnvalue_2 "Local") 0.0 _xlength) (`SplineComponent.GetLocationAtDistanceAlongSpline` _spline _returnvalue_3 "Local") (`KismetMathLibrary.ClampVectorSize` (`SplineComponent.GetTangentAtDistanceAlongSpline` _spline _returnvalue_3 "Local") 0.0 _xlength) true)))