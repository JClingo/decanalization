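; BP_Tile is a level tile whose homeostatic cost falls as actors repeatedly overlap it, shown through a dynamic material's color.
; Each overlap raises a count that divides the base impact, scaled by the game mode's DeltaSeconds, dimming blue.
; BP_GameMode events toggle decanalization, which zeroes impact, changes the count's growth rate and reddens overlapped tiles; recanalization halves the count.
; Reset clears the count and restores blue.
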(event `self.ReceiveBeginPlay`
  (`|ExecutionSequence`
    (:`then_0`
      (bind _returnvalue (`PrimitiveComponent.CreateDynamicMaterialInstance` (`self.Cube`) 0 null "None"))
      (set `self.DynamicMat` _returnvalue))
    (:`then_2`
      (bind _asbp_game_mode (cast `/Game/Agent/BP_GameMode` (`GameplayStatics.GetGameMode`)))
      (set `self.BP Game Mode` _asbp_game_mode))
    (:`then_3`
      (add `/Game/Agent/BP_GameMode.CanalizationToggled` (`self.BP Game Mode`) (delegate `CanalizationToggled_Event`)))
    (:`then_4`
      (add `/Game/Agent/BP_GameMode.Reset` (`self.BP Game Mode`) (delegate `ResetEvent`)))))

(event `CanalizationToggled_Event`
  ; Toggle rate and amount of decanalization
  (if (`/Game/Agent/BP_GameMode.IsDecanalized` (`self.BP Game Mode`))
    (set `self.HomeostaticImpact` 0.0)
    (else
      (set `self.OverlapCount` (`KismetMathLibrary.Conv_IntToDouble` (`KismetMathLibrary.FFloor` (/ (`self.OverlapCount`) 2.0))))
      (bind _output_get (set `self.HomeostaticImpact` (* (/ (`self.BaseHomeostaticImpact`) (+ (`self.OverlapCount`) 1.0)) (`/Game/Agent/BP_GameMode.Delta Seconds` (`self.BP Game Mode`)))))
      (`self.UpdateColor` _output_get))))

(event `ResetEvent`
  (params (ResetTransform :type Boolean))
  ; Reset to initial cost
  (set `self.OverlapCount` 0.0)
  (`MaterialInstanceDynamic.SetVectorParameterValue` (`self.DynamicMat`) "Color" (make `LinearColor` 0.0 0.0 1.0 1.0)))

(event `self.ReceiveActorBeginOverlap`
  (params (OtherActor :type "Actor Object Reference"))
  (`|ExecutionSequence`
    (:`then_0`
      (if (`/Game/Agent/BP_GameMode.IsDecanalized` (`self.BP Game Mode`))
        (set `self.OverlapCount` (+ (`self.OverlapCount`) (`self.DecanalizationRateFactor`)))
        (`self.UpdateColor` (* (/ (`self.BaseHomeostaticImpact`) (+ (`self.OverlapCount`) 1.0)) (`/Game/Agent/BP_GameMode.Delta Seconds` (`self.BP Game Mode`))))
        (else
          (`/Engine/EditorBlueprintResources/StandardMacros.IncrementFloat` (`self.OverlapCount`)
            (:`  `
              ; Decrease cost upon each overlap
              (bind _output_get (set `self.HomeostaticImpact` (* (/ (`self.BaseHomeostaticImpact`) (+ (`self.OverlapCount`) 1.0)) (`/Game/Agent/BP_GameMode.Delta Seconds` (`self.BP Game Mode`)))))
              (`self.UpdateColor` _output_get))))))))

(fn `UpdateColor`
  (params (Impact :type "Float (double-precision)"))
  (bind _bp_game_mode (`self.BP Game Mode`))
  (`MaterialInstanceDynamic.SetVectorParameterValue` (`self.DynamicMat`) "Color" (make `LinearColor` (`KismetMathLibrary.Conv_BoolToDouble` (`/Game/Agent/BP_GameMode.IsDecanalized` _bp_game_mode)) 0.0 (/ (`KismetMathLibrary.SafeDivide` Impact (`self.BaseHomeostaticImpact`)) (* (`/Game/Agent/BP_GameMode.Delta Seconds` _bp_game_mode) 0.75)) 1.0)))

(fn `UserConstructionScript`)