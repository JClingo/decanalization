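; Game mode for a decanalization training experiment that tracks a setpoint distance and logs results per reset cycle to CSV.
; A one-second looping timer averages setpoint history and applies passive loss, while incurred costs lower the setpoint and changes are broadcast.
; Bound events tally harvested rewards and learning-episode results; each reset clears values and appends a row.
; BeginPlay also fixes the random seed, creates the UI and timestamps a file at a hardcoded path.
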(event `SecondElapsed`
  (bind _pastsetpoints (`self.PastSetpoints`))
  (bind _avg (`self.GetFloatArrayAvg` _pastsetpoints))
  ; Log and report setpoint status
  (`|ExecutionSequence`
    (:`then_0`
      (`KismetArrayLibrary.Array_Add` _pastsetpoints (`self.SetpointDistance`))
      (set `self.SetpointAvg` _avg)
      (`self.SetpointAvgChanged` _avg))
    (:`then_1`
      ;; Report passive loss
      (bind _output_get (set `self.SetpointDistance` (- (`self.SetpointDistance`) (`self.PassiveLossRate`))))
      (`self.SetpointChanged` _output_get))
    (:`then_2`
      (`/Engine/EditorBlueprintResources/StandardMacros.IncrementInt` (`self.SecondsElapsed`)))))

(event `self.ReceiveBeginPlay`
  (`|ExecutionSequence`
    (:`then_0`
      (`KismetSystemLibrary.K2_SetTimerDelegate` (delegate `SecondElapsed`) 1.0 true) ; Count seconds elapsed
    )
    (:`then_1`
      (`KismetMathLibrary.SetRandomStreamSeed` (`self.RandomStream`) 1))
    (:`then_2`
      (bind _returnvalue (`|CreateWidget` "/Game/UI/BP_UI.BP_UI_C"))
      (`UserWidget.AddToViewport` _returnvalue 0)
      (set `self.UI` _returnvalue))
    (:`then_3`
      (bind _filename (`self.CreateResultsFile`)) ; Just creates the file--doesn't fill it
      (set `self.File Name` _filename))
    (:`then_4`
      (add `self.Reset` (delegate `ResetEvent`)))
    (:`then_5`
      ; Gather and track rewards harvested
      (add `self.RewardHarvested` (delegate `RewardHarvestedEvent`)))
    (:`then_6`
      (add `self.LearningEpisodeCompleted` (delegate `LearningEpisodeCompletedEvent`)))))

(event `ResetEvent`
  (`self.ResetValues`)
  (`/Engine/EditorBlueprintResources/StandardMacros.IncrementInt` (`self.ResetCount`)
    (:`  `
      (`self.UpdateResultsFile` (`self.File Name`) (`self.ResetCount`) (`self.SetpointAvg`) (`self.RewardsCountForCycle`) (`self.LearningRewardsTotalForCycle`) (`self.StdDevForCycle`) (`self.SecondsElapsed`))
      (set `self.SecondsElapsed` 0)
      (set `self.RewardsCountForCycle` 0)
      (set `self.LearningRewardsTotalForCycle` 0.0))))

(event `RewardHarvestedEvent` :!signature `self.RewardHarvested`
  (params (Reward :type "/Game/Reward/BP_Reward Object Reference"))
  (bind _rewardsharvested (`self.RewardsHarvested`))
  ; Gather and track rewards harvested
  (`BlueprintMapLibrary.Map_Add` _rewardsharvested (+ (`BlueprintMapLibrary.Map_Length` _rewardsharvested) 1) Reward)
  (`/Engine/EditorBlueprintResources/StandardMacros.IncrementInt` (`self.RewardsCountForCycle`)))

(event `LearningEpisodeCompletedEvent` :!signature `self.LearningEpisodeCompleted`
  (params (LearningReward :type "Float (double-precision)") (StandardDeviation :type "Float (double-precision)"))
  (set `self.LearningRewardsTotalForCycle` LearningReward)
  (set `self.StdDevForCycle` StandardDeviation))

(event `CostIncurred`
  (params (Amount :type "Float (double-precision)"))
  (bind _output_get (set `self.SetpointDistance` (- (`self.SetpointDistance`) Amount)))
  (`self.SetpointChanged` _output_get))

(fn `CreateResultsFile`
  (returns (FileName :type String))
  (bind (_returnvalue_year _returnvalue_month _returnvalue_day _returnvalue_hour _returnvalue_minute _returnvalue_second) (`KismetMathLibrary.BreakDateTime` (`KismetMathLibrary.Now`)))
  (bind _returnvalue (`KismetStringLibrary.Concat_StrStr` "C:\\Users\\jingo\\OneDrive\\Work_Cloud\\decanalization\\training-results\\" (`KismetStringLibrary.Conv_IntToString` _returnvalue_year) "-" (`KismetStringLibrary.Conv_IntToString` _returnvalue_month) "-" (`KismetStringLibrary.Conv_IntToString` _returnvalue_day) " at " (`KismetStringLibrary.Conv_IntToString` _returnvalue_hour) "." (`KismetStringLibrary.Conv_IntToString` _returnvalue_minute) "." (`KismetStringLibrary.Conv_IntToString` _returnvalue_second) ".csv"))
  (`FileSDKBPLibrary.CreateFile` _returnvalue)
  (`FileSDKBPLibrary.WriteStringToFile` _returnvalue (`KismetSystemLibrary.MakeLiteralString` (`KismetStringLibrary.Concat_StrStr` "Iteration Count," "Setpoint Average," "Rewards Harvested," "Learning Rewards Given," "Standard Deviation for Setpoints," "Seconds Elapsed," ", \n")))
  (return _returnvalue))

(fn `GetFloatArrayAvg`
  (params (Values :type "Array of Float (double-precision) (by ref)"))
  (returns (Avg :type "Float (double-precision)"))
  (locals (Sum :type "Float (double-precision)"))
  (for _array_element Values
    (set `local.Sum` (+ (`local.Sum`) _array_element)))
  (return (/ (`local.Sum`) (`KismetMathLibrary.Conv_IntToDouble` (`KismetArrayLibrary.Array_Length` Values)))))

(fn `ResetValues`
  (`|ExecutionSequence`
    (:`then_0`
      (bind _output_get (set `self.SetpointDistance` 0.0))
      (`self.SetpointChanged` _output_get)
      (`self.SetpointAvgChanged` 0.0))
    (:`then_1`
      (`KismetArrayLibrary.Array_Clear` (`self.PastSetpoints`)))))

(fn `UpdateResultsFile`
  (params (FileName :type String) (IterationCount :type Integer) (SetpointAvg :type "Float (double-precision)") (RewardsHarvested :type Integer) (LearningRewardsGiven :type "Float (double-precision)") (StandardDeviation :type "Float (double-precision)") (SecondsElapsed :type Integer))
  (`FileSDKBPLibrary.WriteStringToFile` FileName (`KismetSystemLibrary.MakeLiteralString` (`KismetStringLibrary.Concat_StrStr` (`KismetStringLibrary.Conv_IntToString` IterationCount) "," (`KismetStringLibrary.Conv_IntToString` (`KismetMathLibrary.Round` SetpointAvg)) "," (`KismetStringLibrary.Conv_IntToString` RewardsHarvested) "," (`KismetStringLibrary.Conv_IntToString` (`KismetMathLibrary.Round` LearningRewardsGiven)) "," (`KismetStringLibrary.Conv_DoubleToString` StandardDeviation) "," (`KismetStringLibrary.Conv_IntToString` SecondsElapsed) ",, \n")) true))

(fn `UserConstructionScript`)