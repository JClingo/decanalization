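; Game mode for a homeostatic agent experiment, tracking the setpoint, harvests, losses, rewards and locations.
; Impact events and periodic passive loss update the setpoint history; perception updates turn anticipated gains and losses into HRL or LM rewards.
; Trial mode runs tick-timed sequences, toggling canalization in "cdr" order, buffers statistics as YAML, then saves and quits after the last trial.
; Training CSV logging is disconnected.
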(event `self.ReceiveBeginPlay`
  (`|ExecutionSequence`
    (:`then_1`
      (bind _returnvalue (`GameplayStatics.GetActorOfClass` "/Game/Learning/BP_AgentManager.BP_AgentManager_C"))
      (set `self.AgentManager` _returnvalue)
      (if (`KismetSystemLibrary.IsValid` _returnvalue)
        (if (not (`/Game/Learning/BP_AgentManager.Run Inference` _returnvalue))
          (set `self.IsTraining` true))))
    (:`then_2`
      (`KismetMathLibrary.SetRandomStreamSeed` (`self.RandomStream`) 1))
    (:`then_3`
      (bind _returnvalue_2 (`|CreateWidget` "/Game/UI/BP_UI.BP_UI_C"))
      (`UserWidget.AddToViewport` _returnvalue_2 0)
      (set `self.UI` _returnvalue_2))
    (:`then_4`
      (`|ExecutionSequence`
        (:`then_1`
          (if (`self.ShouldLogLifespan`)
            (bind _filename (`self.CreateLogLifespanFile`))
            (set `self.LogFileName` _filename)))))
    (:`then_5`
      (add `self.Reset` (delegate `Reset_Event`)))
    (:`then_6`
      ; Gather and track rewards harvested
      (add `self.ResourceHarvested` (delegate `ResourceHarvestedEvent`)))
    (:`then_7`
      (add `self.ImpactIncurred` (delegate `ImpactIncurred_Event`)))
    (:`then_8`
      (add `self.LearningEpisodeCompleted` (delegate `LearningEpisodeCompleted_Event`)))
    (:`then_9`
      (if (`self.IsTrialMode`)
        (set `self.TrialYML` "--- \ntrials: \n")
        (`self.Reset` true)))
    (:`then_11`
      (add `self.PerceptionUpdated` (delegate `PerceptionUpdated_Event`)))))

(event `ResetTrial_Event`
  (if (`self.IsHRL`)
    (`self.ReadyTrial` (`self.TrialFileName`) (`self.TrialsRun`) "HRL" (`self.TrialSequenceOrder`))
    (else
      (`self.ReadyTrial` (`self.TrialFileName`) (`self.TrialsRun`) "LM" (`self.TrialSequenceOrder`)))))

(event `PerceptionUpdated_Event` :!signature `self.PerceptionUpdated`
  (params (Gains :type "Float (double-precision)") (Losses :type "Float (double-precision)"))
  (bind _netreward (`self.HandlePerception` Gains Losses))
  (set `self.TotalRewards` (+ _netreward (`self.TotalRewards`))))

(event `Reset_Event` :!signature `self.Reset`
  (params (ResetTransform :type Boolean))
  (`self.ResetValues`)
  (if (`self.IsTrialMode`)
    (`self.ResetTrial_Event`)))

(event `ResourceHarvestedEvent` :!signature `self.ResourceHarvested`
  (params (Resource :type "/Game/Resource/BP_Resource Object Reference"))
  (bind _resourcesharvested (`self.ResourcesHarvested`))
  ; Gather and track rewards harvested
  (`BlueprintMapLibrary.Map_Add` _resourcesharvested (+ (`BlueprintMapLibrary.Map_Length` _resourcesharvested) 1) Resource)
  (`/Engine/EditorBlueprintResources/StandardMacros.IncrementInt` (`self.ResourcesHarvestedCountForCycle`)))

(event `ImpactIncurred_Event` :!signature `self.ImpactIncurred`
  (params (Amount :type "Float (double-precision)"))
  (bind _setpoints (`self.Setpoints`))
  (set `self.TotalLoss` (+ Amount (`self.TotalLoss`)))
  (`KismetArrayLibrary.Array_Add` (`self.Setpoints`) (+ (`|GetArrayItem` _setpoints (`KismetArrayLibrary.Array_LastIndex` _setpoints)) Amount))
  (`self.SetpointsChanged`))

(event `LearningEpisodeCompleted_Event` :!signature `self.LearningEpisodeCompleted`
  (params (LearningReward :type "Float (double-precision)") (StandardDeviation :type "Float (double-precision)"))
  (set `self.LearningRewardsTotalForCycle` LearningReward)
  (set `self.LearningSetpointStdDev` StandardDeviation))

(event `self.ReceiveTick`
  (params (DeltaSeconds :type "Float (single-precision)"))
  (bind _setpoints (`self.Setpoints`))
  (set `self.Delta Seconds` DeltaSeconds)
  (`|ExecutionSequence`
    (:`then_0`
      (if (`self.IsTrialMode`)
        (`self.RunTrial` (`self.TrialFileName`) (`KismetStringLibrary.EqualEqual_StrStr` (`self.TrialSequenceOrder`) "cdr"))))
    (:`then_1`
      (if (== (mod (`self.TotalTickCount`) (`self.PeriodTickLength`)) 0)
        ; Log and report setpoint status
        (`|ExecutionSequence`
          (:`then_1`
            (`KismetArrayLibrary.Array_Add` (`self.Setpoints`) (- (`|GetArrayItem` _setpoints (`KismetArrayLibrary.Array_LastIndex` _setpoints)) (`self.PassiveLossRate`)))
            (`self.SetpointsChanged`))
          (:`then_2`
            (`/Engine/EditorBlueprintResources/StandardMacros.IncrementInt` (`self.SecondsElapsed`)))
          (:`then_3`
            (`KismetArrayLibrary.Array_Add` (`self.LocationsTraversed`) (`self.K2_GetActorLocation` (`GameplayStatics.GetPlayerPawn` 0))))
          (:`then_4`
            (set `self.TotalLoss` (+ (`self.TotalLoss`) (`self.PassiveLossRate`))))
          (:`then_5`
            (if (`self.IsTrialMode`)
              _)))))
    (:`then_2`
      (`/Engine/EditorBlueprintResources/StandardMacros.IncrementInt` (`self.TotalTickCount`)
        (:`  `
          (`/Engine/EditorBlueprintResources/StandardMacros.IncrementInt` (`self.TickCountForSequence`)))))))

(event `CanalizationToggled_Event`
  (set `self.IsDecanalized` (not (`self.IsDecanalized`)))
  (`self.CanalizationToggled`))

(fn `CreateLogLifespanFile`
  (returns (FileName :type String))
  (bind (_returnvalue_year _returnvalue_month _returnvalue_day _returnvalue_hour _returnvalue_minute) (`KismetMathLibrary.BreakDateTime` (`KismetMathLibrary.Now`)))
  (bind _returnvalue (`KismetStringLibrary.Concat_StrStr` "C:\\Users\\jingo\\Documents\\Unreal Projects\\decanalization\\logs\\lifespan\\" (`KismetStringLibrary.Conv_IntToString` _returnvalue_year) "-" (`KismetStringLibrary.Conv_IntToString` _returnvalue_month) "-" (`KismetStringLibrary.Conv_IntToString` _returnvalue_day) " at " (`KismetStringLibrary.Conv_IntToString` _returnvalue_hour) "." (`KismetStringLibrary.Conv_IntToString` _returnvalue_minute) ".yaml"))
  (`FileSDKBPLibrary.CreateFile` _returnvalue)
  (`FileSDKBPLibrary.WriteStringToFile` _returnvalue "" false "ForceUTF8")
  (return _returnvalue))

(fn `CreateTrainingResultsFile`
  (returns (FileName :type String))
  (bind (_returnvalue_year _returnvalue_month _returnvalue_day _returnvalue_hour _returnvalue_minute) (`KismetMathLibrary.BreakDateTime` (`KismetMathLibrary.Now`)))
  (bind (_returnvalue_year_2 _returnvalue_month_2 _returnvalue_day_2 _returnvalue_hour_2 _returnvalue_minute_2) (`KismetMathLibrary.BreakDateTime` (`KismetMathLibrary.Now`)))
  (bind _returnvalue (`KismetStringLibrary.Concat_StrStr` "C:\\Users\\jingo\\Documents\\Unreal Projects\\decanalization\\logs\\training\\" (`KismetStringLibrary.Conv_IntToString` _returnvalue_year) "-" (`KismetStringLibrary.Conv_IntToString` _returnvalue_month) "-" (`KismetStringLibrary.Conv_IntToString` _returnvalue_day) " at " (`KismetStringLibrary.Conv_IntToString` _returnvalue_hour) "." (`KismetStringLibrary.Conv_IntToString` _returnvalue_minute) ".csv"))
  ;[0.15 0.1191 0 0.5] Deprecated - CSV
  (`FileSDKBPLibrary.CreateFile` _returnvalue)
  (`FileSDKBPLibrary.WriteStringToFile` _returnvalue (`KismetSystemLibrary.MakeLiteralString` (`KismetStringLibrary.Concat_StrStr` "Iteration," "Setpoint Average," "Resources Harvested," "Net Reward," "Standard Deviation for Setpoints," "Duration (seconds)," ", \n")))
  (return (`KismetStringLibrary.Concat_StrStr` "C:\\Users\\jingo\\Documents\\Unreal Projects\\decanalization\\logs\\training\\" (`KismetStringLibrary.Conv_IntToString` _returnvalue_year_2) "-" (`KismetStringLibrary.Conv_IntToString` _returnvalue_month_2) "-" (`KismetStringLibrary.Conv_IntToString` _returnvalue_day_2) " at " (`KismetStringLibrary.Conv_IntToString` _returnvalue_hour_2) "." (`KismetStringLibrary.Conv_IntToString` _returnvalue_minute_2) ".csv")))

(fn `CreateTrialFile`
  (returns (FileName :type String))
  (locals (FilenameToCreate :type String :default "C:\\Users\\jingo\\Documents\\Unreal Projects\\decanalization\\logs\\tests\\results.yaml") (Filepath :type String :default "C:\\Users\\jingo\\Documents\\Unreal Projects\\decanalization\\logs\\tests\\") (RewardFunction :type String))
  (bind (_returnvalue_year _returnvalue_month _returnvalue_day _returnvalue_hour _returnvalue_minute _returnvalue_second) (`KismetMathLibrary.BreakDateTime` (`KismetMathLibrary.Now`)))
  (bind _returnvalue (`KismetStringLibrary.Concat_StrStr` "C:\\Users\\jingo\\Documents\\Unreal Projects\\decanalization\\logs\\trials\\" (`local.RewardFunction`) "-" (`KismetStringLibrary.ToUpper` (`self.TrialSequenceOrder`)) " at " (`KismetStringLibrary.Concat_StrStr` (`KismetStringLibrary.Conv_IntToString` _returnvalue_year) "-" (`KismetStringLibrary.Conv_IntToString` _returnvalue_month) "-" (`KismetStringLibrary.Conv_IntToString` _returnvalue_day) " at " (`KismetStringLibrary.Conv_IntToString` _returnvalue_hour) "." (`KismetStringLibrary.Conv_IntToString` _returnvalue_minute) "." (`KismetStringLibrary.Conv_IntToString` _returnvalue_second) ".yml")))
  (if (`self.IsHRL`)
    (set `local.RewardFunction` "HRL")
    (else
      (set `local.RewardFunction` "LM")))
  (`FileSDKBPLibrary.CreateFile` _returnvalue false)
  (return _returnvalue))

(fn `GetFloatArrayAvg`
  (params (Values :type "Array of Float (double-precision) (by ref)"))
  (returns (Avg :type "Float (double-precision)"))
  (locals (Sum :type "Float (double-precision)"))
  (for _array_element Values
    (set `local.Sum` (+ (`local.Sum`) _array_element)))
  (return (/ (`local.Sum`) (`KismetMathLibrary.Conv_IntToDouble` (`KismetArrayLibrary.Array_Length` Values)))))

(fn `GetLocationsString`
  (params (InputPin :type "Array of Vector Structure") (SpacePadding :type Integer))
  (returns (LocationsString :type String))
  (locals (CurrentString :type String))
  (if (> (`KismetArrayLibrary.Array_Length` InputPin) 0)
    (for _array_element InputPin
      (set `local.CurrentString` (`KismetStringLibrary.Concat_StrStr` (`local.CurrentString`) " \n"))
      (for _ (range (`local.SpacePadding`))
        (set `local.CurrentString` (`KismetStringLibrary.Concat_StrStr` (`local.CurrentString`) " ")))
      (set `local.CurrentString` (`KismetStringLibrary.Concat_StrStr` (`local.CurrentString`) "- [" (`KismetStringLibrary.Conv_IntToString` (`KismetMathLibrary.Round` (.x _array_element))) ", " (`KismetStringLibrary.Conv_IntToString` (`KismetMathLibrary.Round` (.y _array_element))) "]")))
    (else
      (set `local.CurrentString` "[]")))
  (return (`local.CurrentString`)))

(fn `GetTotalGains`
  (params (Gains :type "Map of Integer to /Game/Resource/BP_Resource Object Reference"))
  (returns (TotalGains :type "Float (double-precision)"))
  (locals (TotalImpact :type "Float (double-precision)"))
  (bind _values (`BlueprintMapLibrary.Map_Values` Gains))
  (for _array_element _values
    (set `local.TotalImpact` (+ (`/Game/Resource/BP_Resource.HomeostaticImpact` _array_element) (`local.TotalImpact`))))
  (return (`local.TotalImpact`)))

(fn `HandlePerception`
  (params (Gains :type "Float (double-precision)") (Losses :type "Float (double-precision)"))
  (returns (NetReward :type "Float (double-precision)"))
  (locals (hHat :type "Float (double-precision)"))
  (bind _setpoints (`self.Setpoints`))
  (bind _anticipatednets (`self.AnticipatedNets`))
  (bind _setpoints_2 (`self.Setpoints`))
  (bind _setpoints_3 (`self.Setpoints`))
  (bind _hhat (`local.hHat`))
  (bind _setpoints_4 (`self.Setpoints`))
  (bind _returnvalue (`KismetArrayLibrary.Array_LastIndex` _setpoints))
  (bind _returnvalue_2 (`KismetMathLibrary.Abs` (`local.hHat`)))
  (bind _returnvalue_3 (+ Gains (* Losses -1.0)))
  (bind _output (`|GetArrayItem` _setpoints_2 (`KismetArrayLibrary.Array_LastIndex` _setpoints_2)))
  (bind _returnvalue_4 (`KismetMathLibrary.Abs` (`|GetArrayItem` _setpoints_4 (`KismetArrayLibrary.Array_LastIndex` _setpoints_4))))
  (bind _returnvalue_5 (- _hhat _output))
  (bind _returnvalue_6 (- _returnvalue_4 _returnvalue_2))
  (if (!= _returnvalue_3 (`|GetArrayItem` _anticipatednets (`KismetArrayLibrary.Array_LastIndex` _anticipatednets)))
    (`KismetArrayLibrary.Array_Add` _anticipatednets _returnvalue_3)
    (set `local.hHat` (+ _returnvalue_3 (`|GetArrayItem` _setpoints_3 (`KismetArrayLibrary.Array_LastIndex` _setpoints_3))))
    (if (`self.IsHRL`)
      ; HRL
      (if (< _returnvalue_2 _returnvalue_4)
        (return (* (`self.PositiveAlpha`) _returnvalue_6))
        (else
          (return (* (`self.NegativeBeta`) _returnvalue_6))))
      (else
        ; LM
        (if (< _output 0.0)
          (if (> _hhat _output)
            (return (* (`self.PositiveAlpha`) _returnvalue_5))
            (else
              (return (* (`self.NegativeBeta`) _returnvalue_5)))))))
    (elif (not (!= (`|GetArrayItem` _setpoints _returnvalue) (`|GetArrayItem` _setpoints (- _returnvalue 1))))
      (return 0.0))))

(fn `ReadyTrial`
  (params (FileName :type String) (TrialId :type Integer) (RewardFunction :type String) (SequenceOrder :type String))
  (locals (FilenameToCreate :type String :default "C:\\Users\\jingo\\Documents\\Unreal Projects\\decanalization\\logs\\results\\results.yaml") (Filepath :type String :default "C:\\Users\\jingo\\Documents\\Unreal Projects\\decanalization\\logs\\results\\"))
  (set `self.TrialYML` (`KismetStringLibrary.Concat_StrStr` (`self.TrialYML`) (`KismetStringLibrary.Concat_StrStr` "- id: " (`KismetStringLibrary.Conv_IntToString` TrialId) "  \n  reward-function: " (`local.RewardFunction`) " \n  sequence-order: " (`local.SequenceOrder`) " \n  sequences: \n")))
  (return))

(fn `ResetValues`
  (bind _setpoints (`self.Setpoints`))
  (bind _anticipatednets (`self.AnticipatedNets`))
  (`|ExecutionSequence`
    (:`then_0`
      (`KismetArrayLibrary.Array_Clear` _setpoints)
      (`KismetArrayLibrary.Array_Add` _setpoints (`KismetMathLibrary.RandomFloatInRangeFromStream` (`self.RandomStream`) -15.0 15.0))
      (`self.SetpointsChanged`))
    (:`then_1`
      (set `self.SecondsElapsed` 0)
      (set `self.ResourcesHarvestedCountForCycle` 0)
      (set `self.LearningRewardsTotalForCycle` 0.0)
      (set `self.TotalRewards` 0.0))
    (:`then_2`
      (`KismetArrayLibrary.Array_Clear` (`self.LocationsTraversed`))
      (`KismetArrayLibrary.Array_Clear` _anticipatednets)
      (`KismetArrayLibrary.Array_Add` _anticipatednets))
    (:`then_3`
      ; Reset Trial Params
      (set `self.TotalTickCount` 0)
      (set `self.TickCountForSequence` 0)
      (set `self.SequenceStateName` "canalized")
      (`BlueprintMapLibrary.Map_Clear` (`self.ResourcesHarvested`))
      (set `self.TotalLoss` 0.0)
      (set `self.SequenceCount` 0))))

(fn `RunTrial`
  (params (Filename :type String) (IsCDR :type Boolean))
  (locals (SequenceDuration :type Integer))
  (bind _resourcesharvested (`self.ResourcesHarvested`))
  (bind _setpoints (`self.Setpoints`))
  (bind _setpoints_2 (`self.Setpoints`))
  (if (<= (`self.TotalTickCount`) 9001)
    (set `local.SequenceDuration` 3000)
    (if (or (== (`self.TotalTickCount`) 3000) (== (`self.TotalTickCount`) 6000) (== (`self.TotalTickCount`) 9000))
      (`/Engine/EditorBlueprintResources/StandardMacros.IncrementInt` (`self.SequenceCount`)
        (:`  `
          (`self.StoreTrial` (`local.Filename`) (`self.SequenceStateName`) (`local.SequenceDuration`) (`self.GetFloatArrayAvg` _setpoints) (`/Game/Libraries/BFL_Common.GetStandardDev` _setpoints) (`self.TotalLoss`) (`BlueprintMapLibrary.Map_Length` _resourcesharvested) (`self.GetTotalGains` _resourcesharvested) (`self.SequenceCount`))
          (`KismetSystemLibrary.PrintString` (`KismetStringLibrary.Concat_StrStr` (`KismetStringLibrary.Conv_IntToString` (+ (`self.TrialsRun`) 1)) " " (`self.SequenceStateName`)))
          ; Reset sequence-specific values
          (`BlueprintMapLibrary.Map_Clear` (`self.ResourcesHarvested`))
          (set `self.TotalLoss` 0.0)
          (set `self.TotalRewards` 0.0)
          (`KismetArrayLibrary.Array_Clear` _setpoints_2)
          (`KismetArrayLibrary.Array_Add` _setpoints_2 (`KismetMathLibrary.RandomFloatInRangeFromStream` (`self.RandomStream`) -15.0 15.0))
          (`self.SetpointsChanged`)
          (if (`local.IsCDR`)
            (if (== (`self.TotalTickCount`) 3000)
              ; Prepare the next state name
              (set `self.SequenceStateName` "decanalized")
              (`self.CanalizationToggled_Event` :!label _label)
              (elif (== (`self.TotalTickCount`) 6000)
                (set `self.SequenceStateName` "recanalized")
                (goto _label)
                (elif (== (`self.TotalTickCount`) 9000)
                  (set `self.SequenceStateName` "canalized"))))))))
    (else
      ; Run n trials and then quit
      (`/Engine/EditorBlueprintResources/StandardMacros.IncrementInt` (`self.TrialsRun`)
        (:`  `
          (if (== (`self.TrialsToRun`) (`self.TrialsRun`))
            (bind _filename (`self.CreateTrialFile`))
            (set `self.TrialFileName` _filename)
            (`self.SaveTrial`)
            (`KismetSystemLibrary.PrintString` "Trials Completed")
            (`KismetSystemLibrary.QuitGame` null "Quit")
            (else
              (`self.Reset` false))))))))

(fn `SaveTrial`
  (`FileSDKBPLibrary.WriteStringToFile` (`self.TrialFileName`) (`self.TrialYML`)))

(fn `StoreTrial`
  (params (FileName :type String) (StateName :type String) (SequenceDuration :type Integer) (AvgSetpoint :type "Float (double-precision)") (SetpointDeviation :type "Float (double-precision)") (LossTotal :type "Float (double-precision)") (GainsHarvested :type Integer) (GainTotal :type "Float (double-precision)") (SequenceIdx :type Integer))
  (set `self.TrialYML` (`KismetStringLibrary.Concat_StrStr` (`self.TrialYML`) (`KismetStringLibrary.Concat_StrStr` "  - state: " StateName " \n    duration: " (`KismetStringLibrary.Conv_IntToString` SequenceDuration) " \n    setpoint-avg: " (`KismetStringLibrary.Conv_DoubleToString` AvgSetpoint) " \n    setpoint-dev: " (`KismetStringLibrary.Conv_DoubleToString` SetpointDeviation) " \n    loss-total: " (`KismetStringLibrary.Conv_DoubleToString` LossTotal) " \n    gains-harvested: " (`KismetStringLibrary.Conv_IntToString` GainsHarvested) " \n    gain-total: " (`KismetStringLibrary.Conv_DoubleToString` GainTotal) " \n    sequence-idx: " (`KismetStringLibrary.Conv_IntToString` SequenceIdx) " \n"))))

(fn `UpdateLogLifespanFile`
  (params (FileName :type String) (SetpointAvg :type "Float (double-precision)") (ResourcesHarvested :type Integer) (StandardDeviation :type "Float (double-precision)") (SecondsElapsed :type Integer) (Locations :type "Array of Vector Structure"))
  (`FileSDKBPLibrary.WriteStringToFile` (`local.FileName`) (`KismetStringLibrary.Concat_StrStr` "---" " \nsetpoint-avg: " (`KismetStringLibrary.Conv_IntToString` (`KismetMathLibrary.Round` SetpointAvg)) " \nresources-harvested: " (`KismetStringLibrary.Conv_IntToString` ResourcesHarvested) " \nsetpoint-std-dev: " (`KismetStringLibrary.Conv_IntToString` (`KismetMathLibrary.Round` StandardDeviation)) " \nduration: " (`KismetStringLibrary.Conv_IntToString` SecondsElapsed) " \nlocations-traversed: " (`self.GetLocationsString` Locations 2)) false "ForceUTF8"))

(fn `UpdateTrainingResultsFile`
  (params (FileName :type String) (IterationCount :type Integer) (SetpointAvg :type "Float (double-precision)") (ResourcesHarvested :type Integer) (LearningRewardsGiven :type "Float (double-precision)") (StandardDeviation :type "Float (double-precision)") (SecondsElapsed :type Integer) (Locations :type "Array of Vector Structure"))
  (`FileSDKBPLibrary.WriteStringToFile` FileName (`KismetStringLibrary.Concat_StrStr` (`KismetStringLibrary.Conv_IntToString` IterationCount) "," (`KismetStringLibrary.Conv_IntToString` (`KismetMathLibrary.Round` SetpointAvg)) "," (`KismetStringLibrary.Conv_IntToString` ResourcesHarvested) "," (`KismetStringLibrary.Conv_DoubleToString` LearningRewardsGiven) "," (`KismetStringLibrary.Conv_IntToString` (`KismetMathLibrary.Round` StandardDeviation)) "," (`KismetStringLibrary.Conv_IntToString` SecondsElapsed) ",, \n") true))

(fn `UserConstructionScript`)