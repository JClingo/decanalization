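; BP_Reward is a respawning pickup that reports to BP_GameMode when harvested.
; Any actor overlap passes LossReduction to the game mode's CostIncurred, then hides the reward, disables its collision and calls CallRewardHarvested with itself.
; A timer set to RespawnRate restores visibility and collision, so the same actor is reused instead of destroyed.
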(event `self.ReceiveBeginPlay`
  (bind _asbp_game_mode (cast `/Game/Character/Blueprints/BP_GameMode` (`GameplayStatics.GetGameMode`)))
  (set `self.BP Game Mode` _asbp_game_mode))

(event `self.ReceiveActorBeginOverlap`
  (params (OtherActor :type "Actor Object Reference"))
  (`|ExecutionSequence`
    (:`then_0`
      (`/Game/Character/Blueprints/BP_GameMode.CostIncurred` (`self.BP Game Mode`) (`self.LossReduction`)))
    (:`then_1`
      (`self.SetActorHiddenInGame` true)
      (`self.SetActorEnableCollision` false)
      (`KismetSystemLibrary.K2_SetTimerDelegate` (delegate `Respawn`) (`self.RespawnRate`)))
    (:`then_2`
      (`/Game/Character/Blueprints/BP_GameMode.RewardHarvested` (`self.BP Game Mode`) self))))

(event `Respawn`
  (`self.SetActorHiddenInGame` false)
  (`self.SetActorEnableCollision` true))

(fn `UserConstructionScript`)